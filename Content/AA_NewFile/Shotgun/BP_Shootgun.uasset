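; BP_Shootgun is a VR grippable shotgun actor that attaches to the controller with a physics constraint.
; On grip, it constrains its physics-simulated mesh to the controller's custom pivot component, using the grip's relative transform as the reference frame.
; Each grip tick, the controller with grip authority drops it if the constraint stretches past a distance limit.
; On release, it breaks the constraint and wakes the mesh's rigid bodies.
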(event EventOnGrip
  (params (GrippingController :type Grip%20Motion%20Controller%20Component%20Object%20Reference) (GripInformation :type BP%20Actor%20Grip%20Information%20Structure%20%28by%20ref%29))
  (bind _grabbingconstraint (Variables|Default|GetGrabbingConstraint))
  (bind _staticmeshcomponent (Variables|Default|GetStaticMeshComponent))
  ;[1 1 1] On Grip
  (|CallParentFunction GrippingController GripInformation)
  (bind _asprimitive_component (Utilities|Casting|CastToPrimitiveComponent (Variables|/Script/VRExpansionPlugin.GripMotionControllerComponent|GetCustomPivotComponent GrippingController)))
  (Class|PhysicsConstraintComponent|SetConstrainedComponents _grabbingconstraint _staticmeshcomponent "None" _asprimitive_component "None")
  (Physics|SetSimulatePhysics _staticmeshcomponent true)
  (Class|PhysicsConstraintComponent|SetConstraintReferenceFrame _grabbingconstraint "Frame2" (.RelativeTransform (Utilities|Struct|BreakBPActorGripInformation GripInformation))))

(event EventOnGripRelease
  (params (ReleasingController :type Grip%20Motion%20Controller%20Component%20Object%20Reference) (GripInformation :type BP%20Actor%20Grip%20Information%20Structure%20%28by%20ref%29) (bWasSocketed :type Boolean))
  ;[1 1 1] On Drop
  (|CallParentFunction ReleasingController GripInformation bWasSocketed)
  (Class|PhysicsConstraintComponent|BreakConstraint (Variables|Default|GetGrabbingConstraint))
  (Class|PrimitiveComponent|WakeAllRigidBodies (Variables|Default|GetStaticMeshComponent)))

(event EventTickGrip
  (params (GrippingController :type Grip%20Motion%20Controller%20Component%20Object%20Reference) (GripInformation :type BP%20Actor%20Grip%20Information%20Structure%20%28by%20ref%29) (DeltaTime :type Float%20%28single-precision%29))
  ;[1 1 1] Distance based dropping on the update grip tick
  (if (Class|GripMotionControllerComponent|HasGripAuthority GrippingController GripInformation)
    (if (> (Math|Vector|VectorLengthSquared (Class|VREPhysicsConstraintComponent|GetCurrentLinearDistance (Variables|Default|GetGrabbingConstraint) "Frame2")) (Math|Float|Square 4e+02))
      (Class|GripMotionControllerComponent|DropObjectbyInterface GrippingController 0 (.GripID (Utilities|Struct|BreakBPActorGripInformation GripInformation)) "0, 0, 0" "0, 0, 0"))))

(fn ConstructionScript)