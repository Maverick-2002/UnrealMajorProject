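; BP_Spawner is an enemy spawner that holds a queue of enemy classes and spawns them at its own transform.
; AddEnemyToQueue appends a class and calls SpawnEnemy at once if no AI_Zombie overlaps its Sphere.
; A looping timer started on BeginPlay also calls SpawnEnemy every minute, without that overlap check.
; SpawnEnemy spawns the first queued class, removes an entry from the queue and returns whether it spawned.
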(event Custom|trytospawn
  (CallFunction|SpawnEnemy))

(event EventBeginPlay
  (Utilities|Time|SetTimerbyEvent (delegate Custom|trytospawn) 6e+01 true))

(event Collision|EventActorBeginOverlap
  (params (OtherActor :type Actor%20Object%20Reference)))

(event EventTick
  (params (DeltaSeconds :type Float%20%28single-precision%29)))

(fn ConstructionScript)

(fn SpawnEnemy
  (if (Utilities|Array|IsValidIndex (Variables|Default|GetEnemyQueue))
    (Game|SpawnActorfromClass (Utilities|Array|Get(acopy) (Variables|Default|GetEnemyQueue)) (Transformation|GetActorTransform) "Undefined" 0 0)
    (Utilities|Array|RemoveItem (Variables|Default|GetEnemyQueue) 0)
    (return true)
    (else
      (return false))))

(fn AddEnemytoQueue
  (params (EnemyClass :type AI%20Zombie%20Class%20Reference%20%28by%20ref%29))
  (Utilities|Array|Add (Variables|Default|GetEnemyQueue) EnemyClass)
  (if (not (Utilities|Array|IsValidIndex (Collision|GetOverlappingActors (Variables|Default|GetSphere) "/Game/AA_NewFile/Character_Enemy_/AI_Zombie.AI_Zombie_C" :!class /Script/Engine.PrimitiveComponent)))
    (CallFunction|SpawnEnemy)))